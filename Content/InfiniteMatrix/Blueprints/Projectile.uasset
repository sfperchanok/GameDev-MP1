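; Projectile actor that flies in a straight line and removes itself on impact or timeout.
; Tick moves it along world X at ForwardSpeed, regardless of its rotation, and destroys it once its accumulated active time passes a fixed lifetime.
; TriggerZone overlap with a BP_Tunnel or Enemy also destroys it; no damage or effect is applied here.
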(event OnComponentBeginOverlap(TriggerZone)
  (params (OverlappedComponent :type Primitive%20Component%20Object%20Reference) (OtherActor :type Actor%20Object%20Reference) (OtherComp :type Primitive%20Component%20Object%20Reference) (OtherBodyIndex :type Integer) (bFromSweep :type Boolean) (SweepResult :type Hit%20Result%20Structure%20%28by%20ref%29))
  (Utilities|Casting|CastToBP_Tunnel OtherActor
    (:then
      _)
    (:CastFailed
      (Utilities|Casting|CastToEnemy OtherActor)))
  (Actor|DestroyActor))

(event EventBeginPlay)

(event Collision|EventActorBeginOverlap
  (params (OtherActor :type Actor%20Object%20Reference)))

(event EventTick
  (params (DeltaSeconds :type Float%20%28single-precision%29))
  (if (> (Variables|Default|GetActiveTime) 5.0)
    (Actor|DestroyActor)
    (else
      (Variables|Default|SetActiveTime (+ DeltaSeconds (Variables|Default|GetActiveTime)))
      (Transformation|AddActorWorldOffset (Math|Vector|MakeVector (* (Variables|Default|GetForwardSpeed) DeltaSeconds) 0.0 0.0)))))

(fn ConstructionScript)